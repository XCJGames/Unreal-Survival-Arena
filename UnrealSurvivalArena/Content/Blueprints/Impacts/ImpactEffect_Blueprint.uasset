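; Impact effect actor that spawns a particle emitter, sound and decal at a hit point when it begins play.
; It builds a decal rotation from the hit normal with random roll, so repeated marks vary.
; A switch on the physical material's surface type has only a default branch, so every surface gets the same effects.
; The decal attaches to the hit component and bone with configurable size and lifespan.
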(event `self.ReceiveBeginPlay`
  (bind _decalsize (`self.DecalSize`))
  (bind (_bblockinghit _binitialoverlap _time _distance _location _impactpoint _normal _impactnormal _physmat _hitactor _hitcomponent _hitbonename) (`GameplayStatics.BreakHitResult` (`self.HitResult`)))
  (`|ExecutionSequence`
    (:`then_0`
      (set `self.RandomDecalRotation` (`KismetMathLibrary.MakeRotator` (`KismetMathLibrary.RandomFloatInRange` -180.0 180.0) (.pitch (`KismetMathLibrary.Conv_VectorToRotator` (`.Normal` (`GameplayStatics.BreakHitResult` (`self.HitResult`))))) (.yaw (`KismetMathLibrary.Conv_VectorToRotator` (`.Normal` (`GameplayStatics.BreakHitResult` (`self.HitResult`))))))))
    (:`then_1`
      (switch `EPhysicalSurface` (`PhysicalMaterial.SurfaceType` _physmat)
        (:`SurfaceType_Default`
          (`GameplayStatics.SpawnEmitterAtLocation` (`self.DefaultFX`) _impactpoint)
          (`GameplayStatics.PlaySoundAtLocation` (`self.DefaultSFX`) _impactpoint (struct) 1.0 1.0 0.0 null null null)
          (`GameplayStatics.SpawnDecalAttached` (`self.DefaultDecalMaterial`) (`KismetMathLibrary.MakeVector` _decalsize _decalsize 1.0) _hitcomponent _hitbonename _impactpoint (`self.RandomDecalRotation`) "KeepRelativeOffset" (`self.DecalLifeSpan`)))))))

(fn `UserConstructionScript`)