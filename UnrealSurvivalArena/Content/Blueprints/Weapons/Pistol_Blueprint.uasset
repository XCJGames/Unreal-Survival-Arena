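; Pistol weapon Blueprint that extends a parent weapon class with pistol-specific firing feedback.
; Shoot runs the parent logic, plays the pistol fire animation on the weapon mesh, spawns a shell-ejection particle at the AmmoEject socket, then increases spread by a fixed amount.
; Reload and the construction script only call their parent implementations.
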(event `self.Reload`
  (`parent.Reload`))

(event `self.Shoot`
  (bind (_returnvalue_location _returnvalue_rotation) (`KismetMathLibrary.BreakTransform` (`SceneComponent.GetSocketTransform` (`self.Weapon`) "AmmoEject" "RTS_World")))
  (`parent.Shoot`)
  (`SkeletalMeshComponent.PlayAnimation` (`self.Weapon`) "/Game/ExternalContent/MilitaryWeapDark/Weapons/Anims/Fire_Pistol_W.Fire_Pistol_W" false)
  (`GameplayStatics.SpawnEmitterAtLocation` "/Game/Effects/ParticleSystems/Weapons/PistolShells_FX.PistolShells_FX" _returnvalue_location _returnvalue_rotation)
  (`self.IncreaseSpread` 0.1))

(fn `UserConstructionScript`
  (`parent.UserConstructionScript`))