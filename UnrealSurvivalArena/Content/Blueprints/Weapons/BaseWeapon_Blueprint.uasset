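; Base weapon Blueprint providing hitscan shooting, magazine and reserve ammo tracking, and aim spread.
; Shoot spends one round, then per burst count line-traces from the player camera within a random spread cone.
; Each trace sends a damage message with ammo data and modifiers to the hit actor, draws a muzzle-to-endpoint beam and spawns impact effects on blocking hits.
; Spread recovers on Tick; StopFire is empty.
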(event `self.ReceiveBeginPlay`
  (set `self.Ammo` (`self.MagSize`)))

(event `self.ReceiveTick`
  (params (DeltaSeconds :type "Float (single-precision)"))
  (if (>= (`self.SpreadCurrent`) (`self.SpreadMin`))
    (`self.DecreaseSpread` (* DeltaSeconds (`self.SpreadDecreaseRate`)))))

(fn `AddDamageTo`
  (params (HitResult :type "HitResult Structure") (EndLocation :type "Vector Structure"))
  (message `/Game/Blueprints/Damageable_Interface.Take Damage` (`.HitActor` (`GameplayStatics.BreakHitResult` HitResult)) (`self.AmmoData`) (`self.MinWeaponDamageModifier`) (`self.MaxWeaponDamageModifier`) (`self.CritDamageModifier`) null HitResult))

(fn `DecreaseSpread`
  (params (DecreaseAmmount :type "Float (double-precision)"))
  (bind _returnvalue (- (`self.SpreadCurrent`) DecreaseAmmount))
  (if (<= _returnvalue (`self.SpreadMin`))
    (set `self.SpreadCurrent` (`self.SpreadMin`))
    (else
      (set `self.SpreadCurrent` _returnvalue))))

(fn `HaveAmmo`
  (returns (`Have Ammo` :type Boolean) (`Have More Ammo Than Mag` :type Boolean))
  (bind _totalammo (`self.TotalAmmo`))
  (return (> _totalammo 0) (> _totalammo (`self.Ammo`))))

(fn `IncreaseSpread`
  (params (IncreaseAmmount :type "Float (double-precision)"))
  (bind _returnvalue (+ IncreaseAmmount (`self.SpreadCurrent`)))
  (if (>= _returnvalue (`self.SpreadMax`))
    (set `self.SpreadCurrent` (`self.SpreadMax`))
    (else
      (set `self.SpreadCurrent` _returnvalue))))

(fn `MagazineIsEmpty`
  (returns (IsEmpty :type Boolean))
  (return (== (`self.Ammo`) 0)))

(fn `MagazineIsFull`
  (returns (IsFull :type Boolean))
  (return (== (`self.Ammo`) (`self.MagSize`))))

(fn `Reload`
  (set `self.Ammo` (`KismetMathLibrary.Min` (`self.MagSize`) (`self.TotalAmmo`))))

(fn `Shoot`
  (bind _weapon (`self.Weapon`))
  (`/Engine/EditorBlueprintResources/StandardMacros.DecrementInt` (`self.Ammo`)
    (:`  `
      (`/Engine/EditorBlueprintResources/StandardMacros.DecrementInt` (`self.TotalAmmo`)
        (:`  `
          (for _ (range 1 (+ (`self.BurstCount`) 1))
            (bind (_projectiletransform _hitresult _endlocation) (`self.ShootInfo` (`/Game/Blueprints/Characters/Player_Blueprint.FirstPersonCamera` (cast `/Game/Blueprints/Characters/Player_Blueprint` (`GameplayStatics.GetPlayerCharacter` 0) :!pure true)) _weapon "MuzzleFlash"))
            (`self.AddDamageTo` _hitresult _endlocation)
            (bind _returnvalue (`GameplayStatics.SpawnEmitterAtLocation` (`self.TrailFX`) (`SceneComponent.GetSocketLocation` _weapon "MuzzleFlash")))
            (`FXSystemComponent.SetVectorParameter` _returnvalue "ShockBeamEnd" _endlocation)
            (bind (_bblockinghit _binitialoverlap _time _distance _location _impactpoint) (`GameplayStatics.BreakHitResult` _hitresult))
            (if _bblockinghit
              (`|SpawnActorFromClass` (`self.ImpactEffect`) (`KismetMathLibrary.Conv_VectorToTransform` _impactpoint) "Undefined" "OverrideRootScale" null _hitresult null))))))))

(fn `ShootInfo`
  (params (Camera :type "CameraComponent Object Reference") (WeaponMesh :type "SceneComponent Object Reference") (MuzzleSocket :type Name))
  (returns (ProjectileTransform :type "Transform Structure") (HitResult :type "HitResult Structure") (EndLocation :type "Vector Structure"))
  (locals (LocalTransform :type "Transform Structure") (LocalEndLocation :type "Vector Structure") (LocalCamera :type "CameraComponent Object Reference") (LocalWeaponMesh :type "SceneComponent Object Reference") (LocalMuzzleSocket :type Name))
  (bind (_returnvalue_location _returnvalue_rotation) (`KismetMathLibrary.BreakTransform` (`SceneComponent.K2_GetComponentToWorld` (`local.LocalCamera`))))
  (bind _returnvalue (`SceneComponent.GetSocketLocation` (`local.LocalWeaponMesh`) (`local.LocalMuzzleSocket`)))
  (bind _returnvalue_2 (+ _returnvalue_location (* (`KismetMathLibrary.RandomUnitVectorInConeInRadians` (`KismetMathLibrary.GetForwardVector` _returnvalue_rotation) (`self.SpreadCurrent`)) 10000.0)))
  (`|ExecutionSequence`
    (:`then_0`
      ;[1 1 1] Setting local variables
      (set `local.LocalCamera` Camera)
      (set `local.LocalWeaponMesh` WeaponMesh)
      (set `local.LocalMuzzleSocket` MuzzleSocket))
    (:`then_1`
      (set `local.LocalEndLocation` _returnvalue_2)
      (bind (_outhit _returnvalue_3) (`KismetSystemLibrary.LineTraceSingleForObjects` _returnvalue_location _returnvalue_2 (`|MakeArray` "ObjectTypeQuery1" "ObjectTypeQuery2" :!type "EObjectTypeQuery Enum") false (`|MakeArray` (`GameplayStatics.GetPlayerPawn` 0) :!type "Actor Object Reference")))
      (if _returnvalue_3
        (bind (_bblockinghit _binitialoverlap _time _distance _location _impactpoint) (`GameplayStatics.BreakHitResult` _outhit))
        (set `local.LocalTransform` (`KismetMathLibrary.MakeTransform` _returnvalue (`KismetMathLibrary.FindLookAtRotation` _returnvalue _impactpoint)))
        (set `local.LocalEndLocation` _impactpoint)
        (else
          (set `local.LocalTransform` (`KismetMathLibrary.MakeTransform` _returnvalue (`Pawn.GetControlRotation` (`GameplayStatics.GetPlayerPawn` 0)))))))
    (:`then_2`
      (return (`local.LocalTransform`) _outhit (`local.LocalEndLocation`)))))

(fn `StopFire`)

(fn `UserConstructionScript`)