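; Rifle weapon Blueprint that provides automatic fire on top of a parent weapon class.
; Shoot fires immediately and starts a looping RifleFire timer at the rifle's fire rate.
; Each shot runs the parent's Shoot, plays the fire animation, increases spread and notifies Player_Blueprint.
; StopFire, also triggered when ammo hits zero, calls the parent's version and clears the timer.
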(event `RifleFire`
  (if (`self.IsRifleFiring`)
    (`parent.Shoot`)
    (`SkeletalMeshComponent.PlayAnimation` (`self.Weapon`) "/Game/ExternalContent/MilitaryWeapDark/Weapons/Anims/Fire_Rifle_W.Fire_Rifle_W" false)
    (`self.IncreaseSpread` 0.1)
    (bind _asplayer_blueprint (cast `/Game/Blueprints/Characters/Player_Blueprint` (`GameplayStatics.GetPlayerCharacter` 0)))
    (`/Game/Blueprints/Characters/Player_Blueprint.OnCharacterShoot` _asplayer_blueprint "NewEnumerator3")
    (if (== (`self.Ammo`) 0)
      (`self.StopFire`))))

(event `self.Shoot`
  (set `self.IsRifleFiring` true)
  (`self.RifleFire`)
  (`KismetSystemLibrary.K2_SetTimer` null "RifleFire" (`self.RiflesFireRate`) true))

(event `self.StopFire`
  (`parent.StopFire`)
  (set `self.IsRifleFiring` false)
  (`KismetSystemLibrary.K2_ClearTimer` null "RifleFire"))

(fn `UserConstructionScript`
  (`parent.UserConstructionScript`))